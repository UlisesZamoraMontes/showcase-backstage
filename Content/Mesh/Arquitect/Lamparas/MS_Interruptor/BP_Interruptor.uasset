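; Light switch actor that toggles up to three referenced lamps and plays a switch sound.
; Overlapping it toggles a component's visibility and enables player input, and leaving reverses both.
; The F key and the ObjectOn event share one path that calls LightOnOff on each lamp.
; Validity checks are nested, so an unset first lamp silences the switch and each later lamp depends on the previous one.
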(event Custom|ObjectOn
  (bind _turnonoff_1 (Variables|Default|GetTurnOnOff_1))
  (bind _turnonoff_2 (Variables|Default|GetTurnOnOff_2))
  (bind _turnonoff_3 (Variables|Default|GetTurnOnOff_3))
  ;[0.1969 0.9331 1] Control of lights
  (Utilities|IsValid _turnonoff_1
    (:Is%20Valid
      ;;[0.6434 0.2294 1] AudioControl
      (Audio|SpawnSoundAttached "/Game/Sounds/Interiors/Sound_Switch.Sound_Switch" (Variables|Default|GetSound_Switch))
      (Default|LightonOff _turnonoff_1)
      (Utilities|IsValid _turnonoff_2
        (:Is%20Valid
          (Default|LightonOff _turnonoff_2)
          (Utilities|IsValid _turnonoff_3
            (:Is%20Valid
              (Default|LightonOff _turnonoff_3))))))))

(event Collision|EventActorBeginOverlap
  (params (OtherActor :type Actor%20Object%20Reference))
  ;[1 0.1106 0.01491] InputControl
  (Rendering|ToggleVisibility false)
  (Input|EnableInput (Game|GetPlayerController 0)))

(event Collision|EventActorEndOverlap
  (params (OtherActor :type Actor%20Object%20Reference))
  ;[1 0.1106 0.01491] InputControl
  (Rendering|ToggleVisibility false)
  (Input|DisableInput (Game|GetPlayerController 0)))

(event Input|KeyboardEvents|F
  (params (Key :type Key%20Structure :default "AnyKey"))
  (bind _turnonoff_1 (Variables|Default|GetTurnOnOff_1))
  (bind _turnonoff_2 (Variables|Default|GetTurnOnOff_2))
  (bind _turnonoff_3 (Variables|Default|GetTurnOnOff_3))
  (:Pressed
    ;[0.1969 0.9331 1] Control of lights
    (Utilities|IsValid _turnonoff_1
      (:Is%20Valid
        ;;[0.6434 0.2294 1] AudioControl
        (Audio|SpawnSoundAttached "/Game/Sounds/Interiors/Sound_Switch.Sound_Switch" (Variables|Default|GetSound_Switch))
        (Default|LightonOff _turnonoff_1)
        (Utilities|IsValid _turnonoff_2
          (:Is%20Valid
            (Default|LightonOff _turnonoff_2)
            (Utilities|IsValid _turnonoff_3
              (:Is%20Valid
                (Default|LightonOff _turnonoff_3)))))))))

(fn ConstructionScript)