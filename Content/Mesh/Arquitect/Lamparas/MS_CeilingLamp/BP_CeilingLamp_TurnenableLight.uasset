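; Ceiling lamp Blueprint with a light that can be switched on and off.
; The construction script creates a dynamic material instance on material slot 0 and stores it for runtime use.
; The LightOnOff event toggles visibility and flips the "Poder de Emision" emission parameter between zero and a lit value, using the current parameter value as the on/off state.
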(event Custom|LightOnOff
  (Rendering|ToggleVisibility false)
  (bind _returnvalue (Rendering|Material|GetScalarParameterValue (Variables|Default|GetDynamic%20Material) "Poder de Emision" :!class /Script/Engine.MaterialInstanceDynamic))
  (if (== _returnvalue 0.0)
    (Rendering|Material|SetScalarParameterValue (Variables|Default|GetDynamic%20Material) "Poder de Emision" 4.0 :!class /Script/Engine.MaterialInstanceDynamic)
    (else
      (Rendering|Material|SetScalarParameterValue (Variables|Default|GetDynamic%20Material) "Poder de Emision" 0.0 :!class /Script/Engine.MaterialInstanceDynamic))))

(fn ConstructionScript
  (bind _returnvalue (Rendering|Material|CreateDynamicMaterialInstance 0 0 :!class /Script/Engine.PrimitiveComponent))
  (Variables|Default|SetDynamic%20Material _returnvalue))