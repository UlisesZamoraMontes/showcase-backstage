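; Player pawn for an asset viewer that orbits, dollies and pans a spring-arm camera around a displayed static mesh.
; Key presses cycle the mesh, render-mode console commands and levels, saving the level index in BP_GameInstanceViewer so the construction script restores it after loading.
; Axis inputs rotate the arm with pitch limits.
; Dolly and offsets use AxisIncrementalStep, a helper whose step accumulates while input is held and resets on release.
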(event EventBeginPlay)

(event Collision|EventActorBeginOverlap
  (params (OtherActor :type Actor%20Object%20Reference)))

(event EventTick
  (params (DeltaSeconds :type Float%20%28single-precision%29)))

(event Input|ActionEvents|InputActionWireframeMode
  (params (Key :type Key%20Structure :default "AnyKey"))
  (:Pressed
    (bind _result (Math|Integer|IncrementInt (Variables|Default|GetIndexRenderMode))
      (:%20%20
        (if (< _result (Utilities|Array|Length (Variables|Default|GetRenderModes)))
          (bind _output_get (Variables|Default|SetIndexRenderMode _result))
          (Development|ExecuteConsoleCommand (Utilities|Array|Get(acopy) (Variables|Default|GetRenderModes) _output_get))
          (else
            (bind _output_get_2 (Variables|Default|SetIndexRenderMode 0))
            (Development|ExecuteConsoleCommand (Utilities|Array|Get(acopy) (Variables|Default|GetRenderModes) _output_get_2))))))))

(event Input|ActionEvents|InputActionChangeLevel
  (params (Key :type Key%20Structure :default "AnyKey"))
  (:Pressed
    (bind _result (Math|Integer|IncrementInt (Variables|Default|GetIndexLevel))
      (:%20%20
        (if (< _result (Utilities|Array|Length (Variables|Default|GetLevels)))
          (bind _output_get (Variables|Default|SetIndexLevel _result))
          (bind _asbp_game_instance_viewer (Utilities|Casting|CastToBP_GameInstanceViewer (Game|GetGameInstance)))
          (Variables|/Game/Blueprints/BP_GameInstanceViewer.BP_GameInstanceViewer_C|SetPlayerCurrentLevel _asbp_game_instance_viewer _output_get)
          (Game|OpenLevel(byName) (Utilities|Array|Get(acopy) (Variables|Default|GetLevels) _output_get))
          (else
            (bind _output_get_2 (Variables|Default|SetIndexLevel 0))
            (bind _asbp_game_instance_viewer_2 (Utilities|Casting|CastToBP_GameInstanceViewer (Game|GetGameInstance)))
            (Variables|/Game/Blueprints/BP_GameInstanceViewer.BP_GameInstanceViewer_C|SetPlayerCurrentLevel _asbp_game_instance_viewer_2 0)
            (Game|OpenLevel(byName) (Utilities|Array|Get(acopy) (Variables|Default|GetLevels) _output_get_2))))))))

(event Input|ActionEvents|InputActionChangeAsset
  (params (Key :type Key%20Structure :default "AnyKey"))
  (:Pressed
    (bind _result (Math|Integer|IncrementInt (Variables|Default|GetIndexAsset))
      (:%20%20
        (if (< _result (Utilities|Array|Length (Variables|Default|GetAssetsList)))
          (bind _output_get (Variables|Default|SetIndexAsset _result))
          (Components|StaticMesh|SetStaticMesh (Variables|Default|GetSM_InDisplay) (Utilities|Array|Get(acopy) (Variables|Default|GetAssetsList) _output_get))
          (else
            (Variables|Default|SetIndexAsset 0)
            (Components|StaticMesh|SetStaticMesh (Variables|Default|GetSM_InDisplay) (Utilities|Array|Get(acopy) (Variables|Default|GetAssetsList)))))))))

(event Input|AxisEvents|InputAxisHorizontalCameraOffset
  (params (AxisValue :type Float%20%28single-precision%29))
  (bind _camera (Variables|Default|GetCamera))
  (bind _relativelocation (Variables|/Script/Engine.SceneComponent|GetRelativeLocation _camera))
  (bind (_floatincremented _finishincrementalstep) (CallFunction|AxisIncrementalStep AxisValue (.y _relativelocation) (Variables|Default|GetHorizontalOffsetIncrementalStep)))
  (Transformation|SetRelativeLocation (Variables|Default|GetCamera) (Math|Vector|MakeVector (.x _relativelocation) _floatincremented (.z _relativelocation)) false false)
  (Variables|Default|SetHorizontalOffsetIncrementalStep _finishincrementalstep))

(event Input|AxisEvents|InputAxisDollySpringArm
  (params (AxisValue :type Float%20%28single-precision%29))
  (Variables|Default|SetCurrentDollyDistance (Variables|/Script/Engine.SpringArmComponent|GetTargetArmLength (Variables|Default|GetSpringArm)))
  (bind (_floatincremented _finishincrementalstep) (CallFunction|AxisIncrementalStep AxisValue (Variables|/Script/Engine.SpringArmComponent|GetTargetArmLength (Variables|Default|GetSpringArm)) (Variables|Default|GetDollyIncrementalStep)))
  (Variables|/Script/Engine.SpringArmComponent|SetTargetArmLength (Variables|Default|GetSpringArm) _floatincremented)
  (Variables|Default|SetDollyIncrementalStep _finishincrementalstep))

(event Input|AxisEvents|InputAxisCameraVerticalRotate
  (params (AxisValue :type Float%20%28single-precision%29))
  (bind _springarm (Variables|Default|GetSpringArm))
  (bind _output_get (Variables|Default|SetCurrentSpringArmRotation (Variables|/Script/Engine.SceneComponent|GetRelativeRotation _springarm)))
  (if (and (<= (.Pitch (Math|Rotator|BreakRotator _output_get)) (Variables|Default|GetVerticalBottomSpringArmTreshold)) (>= (.Pitch (Math|Rotator|BreakRotator _output_get)) (Variables|Default|GetVerticalTopSpringArmTreshold)))
    (bind _output_get_2 (Variables|Default|SetNewSpringArmRotation (Math|Rotator|MakeRotator (.roll (Variables|Default|GetCurrentSpringArmRotation)) (+ (.pitch (Variables|Default|GetCurrentSpringArmRotation)) AxisValue) (.yaw (Variables|Default|GetCurrentSpringArmRotation)))))
    (Transformation|SetRelativeRotation _springarm _output_get_2 false false)
    (elif (>= (.Pitch (Math|Rotator|BreakRotator _output_get)) (Variables|Default|GetVerticalTopSpringArmTreshold))
      (bind _output_get_3 (Variables|Default|SetNewSpringArmRotation (Math|Rotator|MakeRotator (.roll (Variables|Default|GetCurrentSpringArmRotation)) (- (Variables|Default|GetVerticalBottomSpringArmTreshold) 1.0) (.yaw (Variables|Default|GetCurrentSpringArmRotation)))))
      (Transformation|SetRelativeRotation _springarm _output_get_3 false false)
      (else
        (bind _output_get_4 (Variables|Default|SetNewSpringArmRotation (Math|Rotator|MakeRotator (.roll (Variables|Default|GetCurrentSpringArmRotation)) (+ (Variables|Default|GetVerticalTopSpringArmTreshold) 1.0) (.yaw (Variables|Default|GetCurrentSpringArmRotation)))))
        (Transformation|SetRelativeRotation _springarm _output_get_4 false false)))))

(event Input|AxisEvents|InputAxisVerticalCameraOffset
  (params (AxisValue :type Float%20%28single-precision%29))
  (bind _springarm (Variables|Default|GetSpringArm))
  (Variables|Default|SetCurrentSpringArmTargetOffset (Variables|/Script/Engine.SpringArmComponent|GetTargetOffset _springarm))
  (bind (_floatincremented _finishincrementalstep) (CallFunction|AxisIncrementalStep AxisValue (.z (Variables|/Script/Engine.SpringArmComponent|GetTargetOffset _springarm)) (Variables|Default|GetVerticalOffsetIncrementalStep)))
  (Variables|/Script/Engine.SpringArmComponent|SetTargetOffset _springarm (Math|Vector|MakeVector (.x (Variables|/Script/Engine.SpringArmComponent|GetTargetOffset _springarm)) (.y (Variables|/Script/Engine.SpringArmComponent|GetTargetOffset _springarm)) _floatincremented))
  (Variables|Default|SetVerticalOffsetIncrementalStep _finishincrementalstep))

(event Input|AxisEvents|InputAxisHorizontalRotationSpringArm
  (params (AxisValue :type Float%20%28single-precision%29))
  (bind _springarm (Variables|Default|GetSpringArm))
  (Variables|Default|SetCurrentSpringArmRotation (Variables|/Script/Engine.SceneComponent|GetRelativeRotation _springarm))
  (bind _output_get (Variables|Default|SetNewSpringArmRotation (Math|Rotator|MakeRotator (.roll (Variables|Default|GetCurrentSpringArmRotation)) (.pitch (Variables|Default|GetCurrentSpringArmRotation)) (+ (.yaw (Variables|Default|GetCurrentSpringArmRotation)) AxisValue))))
  (Transformation|SetRelativeRotation _springarm _output_get false false))

(fn ConstructionScript
  (Components|StaticMesh|SetStaticMesh (Variables|Default|GetSM_InDisplay) (Utilities|Array|Get(acopy) (Variables|Default|GetAssetsList) (Variables|Default|GetIndexAsset)))
  (bind _asbp_game_instance_viewer (Utilities|Casting|CastToBP_GameInstanceViewer (Game|GetGameInstance)))
  (Variables|Default|SetIndexLevel (Variables|/Game/Blueprints/BP_GameInstanceViewer.BP_GameInstanceViewer_C|GetPlayerCurrentLevel _asbp_game_instance_viewer)))

(fn AxisIncrementalStep
  (params (AxisFloat :type Float%20%28single-precision%29) (FloatToIncrement :type Float%20%28single-precision%29) (CurrentIncrementalStep :type Float%20%28single-precision%29))
  (bind _returnvalue (+ CurrentIncrementalStep AxisFloat))
  (if (or (> AxisFloat 0.0) (< AxisFloat 0.0))
    (return (+ FloatToIncrement _returnvalue) (* _returnvalue (Math|Float|Absolute(Float) AxisFloat)))
    (else
      (return FloatToIncrement 0.0))))