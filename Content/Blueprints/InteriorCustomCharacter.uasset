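; Player character for a touch-driven interior walkthrough that lets the player switch on household objects.
; Axis inputs drive walking and looking, with rate-based look axes scaled by frame time.
; The ShotRaycast action traces the Visibility channel under the first finger and casts the hit actor in turn to TV, fireplace, table lamp or switch Blueprints, calling ObjectOn on the match.
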(event Input|ActionEvents|InputActionShotRaycast
  (params (Key :type Key%20Structure :default "AnyKey"))
  (bind _returnvalue (Game|GetPlayerController 0))
  (bind _hitresult (Class|PlayerController|GetHitResultUnderFingerbyChannel _returnvalue "Touch1" "TraceTypeQuery1" true))
  (bind _hitactor (Collision|BreakHitResult _hitresult))
  (:Pressed
    (Utilities|IsValid _hitactor
      (:Is%20Valid
        (bind _asms_tv_sony_blueprint (Utilities|Casting|CastToMS_TV_Sony_Blueprint _hitactor)
          (:then
            (Default|Objecton _asms_tv_sony_blueprint))
          (:CastFailed
            (bind _asms_fireplace_030_blueprint (Utilities|Casting|CastToMS_Fireplace_030_Blueprint _hitactor)
              (:then
                (Default|Objecton _asms_fireplace_030_blueprint))
              (:CastFailed
                (bind _asms_table_lamp_b_blueprint (Utilities|Casting|CastToMS_TableLampB_Blueprint _hitactor)
                  (:then
                    (Default|Objecton _asms_table_lamp_b_blueprint))
                  (:CastFailed
                    (bind _asbp_interruptor (Utilities|Casting|CastToBP_Interruptor _hitactor))
                    (Default|Objecton _asbp_interruptor)))))))))))

(event Input|AxisEvents|InputAxisTurn
  (params (AxisValue :type Float%20%28single-precision%29))
  (Pawn|Input|AddControllerYawInput AxisValue))

(event Input|AxisEvents|InputAxisLookUp
  (params (AxisValue :type Float%20%28single-precision%29))
  (Pawn|Input|AddControllerPitchInput AxisValue))

(event Input|AxisEvents|InputAxisMoveForward
  (params (AxisValue :type Float%20%28single-precision%29))
  (Pawn|Input|AddMovementInput (Transformation|GetActorForwardVector) AxisValue false))

(event Input|AxisEvents|InputAxisMoveRight
  (params (AxisValue :type Float%20%28single-precision%29))
  (Pawn|Input|AddMovementInput (Transformation|GetActorRightVector) AxisValue false))

(event Input|AxisEvents|InputAxisTurnRate
  (params (AxisValue :type Float%20%28single-precision%29))
  (Pawn|Input|AddControllerYawInput (* AxisValue 1.0 (Utilities|Time|GetWorldDeltaSeconds))))

(event Input|AxisEvents|InputAxisLookUpRate
  (params (AxisValue :type Float%20%28single-precision%29))
  (Pawn|Input|AddControllerPitchInput (* AxisValue 1.0 (Utilities|Time|GetWorldDeltaSeconds))))

(fn ConstructionScript)