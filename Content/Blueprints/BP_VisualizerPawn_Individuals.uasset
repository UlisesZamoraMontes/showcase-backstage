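; Visualizer pawn that displays one static mesh at a time from an asset list for individual viewing.
; Construction sets the mesh at the current index, and BeginPlay creates and shows the WBP_Individuals widget.
; ChangeAssetWiget steps to the next mesh, wrapping to the first after the last.
; A LevelChanged binding removes all widgets when that event fires.
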(event Custom|ChangeAssetWiget
  (bind _result (Math|Integer|IncrementInt (Variables|Default|GetIndexAsset))
    (:%20%20
      (if (< _result (Utilities|Array|Length (Variables|Default|GetAssetsList)))
        (bind _output_get (Variables|Default|SetIndexAsset _result))
        (Components|StaticMesh|SetStaticMesh (Variables|Default|GetSM_InDisplay) (Utilities|Array|Get(acopy) (Variables|Default|GetAssetsList) _output_get))
        (else
          (Variables|Default|SetIndexAsset 0)
          (Components|StaticMesh|SetStaticMesh (Variables|Default|GetSM_InDisplay) (Utilities|Array|Get(acopy) (Variables|Default|GetAssetsList))))))))

(event Custom|RevomeWBP
  (Viewport|RemoveAllWidgets))

(event EventBeginPlay
  (|CallParentFunction)
  (bind _returnvalue (UserInterface|CreateWidget "/Game/Blueprints/WBP_Individuals.WBP_Individuals_C"))
  (bind _output_get (Variables|Default|SetWBP_indivudualsRef _returnvalue))
  (UserInterface|Viewport|AddtoViewport _output_get 0)
  (EventDispatchers|BindEventtoLevelChanged (delegate Custom|RevomeWBP)))

(event Collision|EventActorBeginOverlap
  (params (OtherActor :type Actor%20Object%20Reference)))

(event EventTick
  (params (DeltaSeconds :type Float%20%28single-precision%29)))

(fn ConstructionScript
  (|CallParentFunction)
  (Components|StaticMesh|SetStaticMesh (Variables|Default|GetSM_InDisplay) (Utilities|Array|Get(acopy) (Variables|Default|GetAssetsList) (Variables|Default|GetIndexAsset))))