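; Player pawn for a touch-driven visualizer, with an orbit camera, HUD, level cycling and playback of a level sequence.
; Axis inputs rotate, dolly and offset the spring-arm camera; AxisIncrementalStep makes dolly and offsets build up while input is held.
; A touch trace opens material or geometry info widgets for the hit object.
; BeginPlay picks the next level from Levels for ChangeLevelHud, and StartSecuencerTouch plays the sequence or skips to its end.
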(event Custom|ChangeLevelHud
  (Game|OpenLevel(byName) (Variables|Default|GetNextLevelName))
  (Default|CallLevelChanged))

(event Custom|StartSecuencerTouch
  (bind _levelsequencer (Variables|Default|GetLevelSequencer))
  (Utilities|IsValid _levelsequencer
    (:Is%20Valid
      (Utilities|IsValid (Variables|Default|GetLevelSequencerPlayer)
        (:Is%20Valid
          (if (Audio|Components|Audio|IsPlaying (Variables|Default|GetLevelSequencerPlayer))
            (Components|Timeline|SetPlaybackPosition (Variables|Default|GetLevelSequencerPlayer) (Class|LevelSequencePlayer|GetLength (Variables|Default|GetLevelSequencerPlayer)))
            (else
              (Components|Timeline|SetPlaybackPosition (Variables|Default|GetLevelSequencerPlayer) 0.0)
              (Audio|Components|Audio|Play (Variables|Default|GetLevelSequencerPlayer)))))
        (:Is%20Not%20Valid
          (bind _returnvalue (Sequencer|Player|CreateLevelSequencePlayer _levelsequencer))
          (bind _output_get (Variables|Default|SetLevelSequencerPlayer _returnvalue))
          (Audio|Components|Audio|Play _output_get))))))

(event Collision|EventActorBeginOverlap
  (params (OtherActor :type Actor%20Object%20Reference)))

(event EventTick
  (params (DeltaSeconds :type Float%20%28single-precision%29)))

(event EventBeginPlay
  (bind _levels (Variables|Default|GetLevels))
  (bind _returnvalue (UserInterface|CreateWidget "/Game/Blueprints/WBP_HUD.WBP_HUD_C"))
  (bind _output_get (Variables|Default|SetHUD_ref _returnvalue))
  (UserInterface|Viewport|AddtoViewport _output_get 0)
  (bind _index (Utilities|FlowControl|ForLoopwithBreak 0 (- (Utilities|Array|Length (Variables|Default|GetLevels)) 1) :!label _label)
    (:LoopBody
      (bind _returnvalue_2 (Game|GetCurrentLevelName true))
      (if (and (Utilities|Name|Equal(Name) (Utilities|String|StringToName _returnvalue_2) (Utilities|Array|Get(acopy) _levels _index)) (Utilities|Name|NotEqual(Name) (Utilities|String|StringToName _returnvalue_2) (Utilities|Array|Get(acopy) _levels (- (Utilities|Array|Length _levels) 1))))
        (Variables|Default|SetNextLevelName (Utilities|Array|Get(acopy) (Variables|Default|GetLevels) (+ _index 1)))
        (goto _label Break)
        (else
          (Variables|Default|SetNextLevelName (Utilities|Array|Get(acopy) (Variables|Default|GetLevels))))))))

(event Input|ActionEvents|InputActionShotRaycast
  (params (Key :type Key%20Structure :default "AnyKey"))
  (bind _returnvalue (Game|GetPlayerController 0))
  (bind _hitresult (Class|PlayerController|GetHitResultUnderFingerbyChannel _returnvalue "Touch1" "TraceTypeQuery1" true))
  (bind _hitactor (Collision|BreakHitResult _hitresult))
  (:Pressed
    (Utilities|IsValid _hitactor
      (:Is%20Valid
        (bind _asbp_material_object (Utilities|Casting|CastToBP_MaterialObject _hitactor)
          (:then
            (bind _returnvalue_2 (UserInterface|CreateWidget "/Game/Blueprints/WBP_MaterialInfo.WBP_MaterialInfo_C"))
            (Variables|/Game/Blueprints/WBP_MaterialInfo.WBP_MaterialInfo_C|SetBaseObject _returnvalue_2 _asbp_material_object)
            (Default|CreateMaterialsUmg _returnvalue_2)
            (UserInterface|Viewport|AddtoViewport _returnvalue_2 0))
          (:CastFailed
            (bind _asbp_geometry_object (Utilities|Casting|CastToBP_GeometryObject _hitactor))
            (bind _returnvalue_3 (UserInterface|CreateWidget "/Game/Blueprints/WBP_GeometryInfo.WBP_GeometryInfo_C"))
            (Variables|/Game/Blueprints/WBP_GeometryInfo.WBP_GeometryInfo_C|SetGeometryObject _returnvalue_3 _asbp_geometry_object)
            (Default|CreateGeometryUmg _returnvalue_3)
            (UserInterface|Viewport|AddtoViewport _returnvalue_3 0)))))))

(event Input|AxisEvents|InputAxisHorizontalCameraOffset
  (params (AxisValue :type Float%20%28single-precision%29))
  (bind _offsetcameratreshold (Variables|Default|GetOffsetCameraTreshold))
  (bind _camera (Variables|Default|GetCamera))
  (bind _relativelocation (Variables|/Script/Engine.SceneComponent|GetRelativeLocation _camera))
  (bind (_floatincremented _finishincrementalstep) (CallFunction|AxisIncrementalStep AxisValue (.y _relativelocation) (Variables|Default|GetHorizontalOffsetIncrementalStep)))
  (Transformation|SetRelativeLocation (Variables|Default|GetCamera) (Math|Vector|MakeVector (.x _relativelocation) (Math|Float|Clamp(Float) _floatincremented (* -1 (.y _offsetcameratreshold)) (.y _offsetcameratreshold)) (.z _relativelocation)) false false)
  (Variables|Default|SetHorizontalOffsetIncrementalStep _finishincrementalstep))

(event Input|AxisEvents|InputAxisDollySpringArm
  (params (AxisValue :type Float%20%28single-precision%29))
  (Variables|Default|SetCurrentDollyDistance (Variables|/Script/Engine.SpringArmComponent|GetTargetArmLength (Variables|Default|GetSpringArm)))
  (bind (_floatincremented _finishincrementalstep) (CallFunction|AxisIncrementalStep AxisValue (Variables|/Script/Engine.SpringArmComponent|GetTargetArmLength (Variables|Default|GetSpringArm)) (Variables|Default|GetDollyIncrementalStep)))
  (Variables|/Script/Engine.SpringArmComponent|SetTargetArmLength (Variables|Default|GetSpringArm) _floatincremented)
  (Variables|Default|SetDollyIncrementalStep _finishincrementalstep))

(event Input|AxisEvents|InputAxisCameraVerticalRotate
  (params (AxisValue :type Float%20%28single-precision%29))
  (Variables|Default|SetCurrentSpringArmRotation (Variables|/Script/Engine.SceneComponent|GetRelativeRotation (Variables|Default|GetSpringArm)))
  (bind _output_get (Variables|Default|SetNewSpringArmRotation (Math|Rotator|MakeRotator (.roll (Variables|Default|GetCurrentSpringArmRotation)) (Math|Float|Clamp(Float) (+ (.pitch (Variables|Default|GetCurrentSpringArmRotation)) AxisValue) (Variables|Default|GetVerticalTopSpringArmTreshold) (Variables|Default|GetVerticalBottomSpringArmTreshold)) (.yaw (Variables|Default|GetCurrentSpringArmRotation)))))
  (Transformation|SetRelativeRotation (Variables|Default|GetSpringArm) _output_get false false))

(event Input|AxisEvents|InputAxisVerticalCameraOffset
  (params (AxisValue :type Float%20%28single-precision%29))
  (bind _offsetcameratreshold (Variables|Default|GetOffsetCameraTreshold))
  (bind _springarm (Variables|Default|GetSpringArm))
  (Variables|Default|SetCurrentSpringArmTargetOffset (Variables|/Script/Engine.SpringArmComponent|GetTargetOffset _springarm))
  (bind (_floatincremented _finishincrementalstep) (CallFunction|AxisIncrementalStep AxisValue (.z (Variables|/Script/Engine.SpringArmComponent|GetTargetOffset _springarm)) (Variables|Default|GetVerticalOffsetIncrementalStep)))
  (Variables|/Script/Engine.SpringArmComponent|SetTargetOffset _springarm (Math|Vector|MakeVector (.x (Variables|/Script/Engine.SpringArmComponent|GetTargetOffset _springarm)) (.y (Variables|/Script/Engine.SpringArmComponent|GetTargetOffset _springarm)) (Math|Float|Clamp(Float) _floatincremented (* -1 (.z _offsetcameratreshold)) (.z _offsetcameratreshold))))
  (Variables|Default|SetVerticalOffsetIncrementalStep _finishincrementalstep))

(event Input|AxisEvents|InputAxisHorizontalRotationSpringArm
  (params (AxisValue :type Float%20%28single-precision%29))
  (bind _springarm (Variables|Default|GetSpringArm))
  (Variables|Default|SetCurrentSpringArmRotation (Variables|/Script/Engine.SceneComponent|GetRelativeRotation _springarm))
  (bind _output_get (Variables|Default|SetNewSpringArmRotation (Math|Rotator|MakeRotator (.roll (Variables|Default|GetCurrentSpringArmRotation)) (.pitch (Variables|Default|GetCurrentSpringArmRotation)) (+ (.yaw (Variables|Default|GetCurrentSpringArmRotation)) AxisValue))))
  (Transformation|SetRelativeRotation _springarm _output_get false false))

(fn ConstructionScript
  (bind _asbp_game_instance_viewer (Utilities|Casting|CastToBP_GameInstanceViewer (Game|GetGameInstance)))
  (Variables|Default|SetIndexLevel (Variables|/Game/Blueprints/BP_GameInstanceViewer.BP_GameInstanceViewer_C|GetPlayerCurrentLevel _asbp_game_instance_viewer)))

(fn AxisIncrementalStep
  (params (AxisFloat :type Float%20%28single-precision%29) (FloatToIncrement :type Float%20%28single-precision%29) (CurrentIncrementalStep :type Float%20%28single-precision%29))
  (bind _returnvalue (+ CurrentIncrementalStep AxisFloat))
  (if (or (> AxisFloat 0.0) (< AxisFloat 0.0))
    (return (+ FloatToIncrement _returnvalue) (* _returnvalue (Math|Float|Absolute(Float) AxisFloat)))
    (else
      (return FloatToIncrement 0.0))))