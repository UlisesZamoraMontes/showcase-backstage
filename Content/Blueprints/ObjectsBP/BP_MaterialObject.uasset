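; Actor Blueprint for a static mesh object whose material can be switched from an array of material entries.
; The construction script applies the configured mesh to SMObject, along with the material at the current MaterialIndex.
; The ChangeMaterial event reapplies slot 0 from that index, resetting to the first entry when the index is out of range.
; It does not advance the index itself.
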(event Custom|ChangeMaterial
  (if (Utilities|Array|IsValidIndex (Variables|Default|GetMaterialInformation) (Variables|Default|GetMaterialIndex))
    (Rendering|Material|SetMaterial (Variables|Default|GetSM_Object) 0 (.Material (Utilities|Struct|BreakMaterialBase (Utilities|Array|Get(acopy) (Variables|Default|GetMaterialInformation) (Variables|Default|GetMaterialIndex)))))
    (else
      (bind _output_get (Variables|Default|SetMaterialIndex 0))
      (Rendering|Material|SetMaterial (Variables|Default|GetSM_Object) 0 (.Material (Utilities|Struct|BreakMaterialBase (Utilities|Array|Get(acopy) (Variables|Default|GetMaterialInformation) _output_get)))))))

(event EventBeginPlay)

(event Collision|EventActorBeginOverlap
  (params (OtherActor :type Actor%20Object%20Reference)))

(event EventTick
  (params (DeltaSeconds :type Float%20%28single-precision%29)))

(fn ConstructionScript
  (bind _sm_object (Variables|Default|GetSM_Object))
  (Components|StaticMesh|SetStaticMesh _sm_object (Variables|Default|GetMeshToShow))
  (Rendering|Material|SetMaterial _sm_object 0 (.Material (Utilities|Struct|BreakMaterialBase (Utilities|Array|Get(acopy) (Variables|Default|GetMaterialInformation) (Variables|Default|GetMaterialIndex))))))