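; BP_GeometryObject is an actor whose static mesh is chosen from the GeometryInformation array by GeometryIndex.
; The construction script applies the indexed mesh to SMObject.
; The ChangeGeometry event reapplies it, resetting an invalid index to zero first, but does not advance the index itself.
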(event Custom|ChangeGeometry
  (if (Utilities|Array|IsValidIndex (Variables|Default|GetGeometryInformation) (Variables|Default|GetGeometryIndex))
    (Components|StaticMesh|SetStaticMesh (Variables|Default|GetSM_Object) (.Geometry (Utilities|Struct|BreakGeometryBase (Utilities|Array|Get(acopy) (Variables|Default|GetGeometryInformation) (Variables|Default|GetGeometryIndex)))))
    (else
      (bind _output_get (Variables|Default|SetGeometryIndex 0))
      (Components|StaticMesh|SetStaticMesh (Variables|Default|GetSM_Object) (.Geometry (Utilities|Struct|BreakGeometryBase (Utilities|Array|Get(acopy) (Variables|Default|GetGeometryInformation) _output_get)))))))

(event EventBeginPlay)

(event Collision|EventActorBeginOverlap
  (params (OtherActor :type Actor%20Object%20Reference)))

(event EventTick
  (params (DeltaSeconds :type Float%20%28single-precision%29)))

(fn ConstructionScript
  (Components|StaticMesh|SetStaticMesh (Variables|Default|GetSM_Object) (.Geometry (Utilities|Struct|BreakGeometryBase (Utilities|Array|Get(acopy) (Variables|Default|GetGeometryInformation) (Variables|Default|GetGeometryIndex))))))